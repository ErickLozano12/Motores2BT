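; Traffic light actor that cycles its lights and gates BP_SplineRuta actors entering its trigger box.
; ChangeTrafficLightState starts at BeginPlay, shows one light, stores the next state in TrafficState and re-arms itself by timer, cycling red, green, yellow.
; On box overlap, it clears CanMove when TrafficState is Verde (red showing) and sets it otherwise.
; The check runs only on entry, so light changes never release stopped actors here.
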(event OnComponentBeginOverlap(Box)
  (params (OverlappedComponent :type Primitive%20Component%20Object%20Reference) (OtherActor :type Actor%20Object%20Reference) (OtherComp :type Primitive%20Component%20Object%20Reference) (OtherBodyIndex :type Integer) (bFromSweep :type Boolean) (SweepResult :type Hit%20Result%20Structure%20%28by%20ref%29))
  (Development|PrintString "NPC ENTRO AL TRIGGER")
  (bind _asbp_spline_ruta (Utilities|Casting|CastToBP_SplineRuta OtherActor))
  (if (Utilities|Enum|Equal(Enum) (Variables|Default|GetTrafficState) "NewEnumerator2")
    (Variables|/Game/Characters/AI/BP_SplineRuta.BP_SplineRuta_C|SetbCanMove _asbp_spline_ruta false)
    (else
      (Variables|/Game/Characters/AI/BP_SplineRuta.BP_SplineRuta_C|SetbCanMove _asbp_spline_ruta true)
      (Development|PrintString "npcDetenido"))))

(event OnComponentEndOverlap(Box)
  (params (OverlappedComponent :type Primitive%20Component%20Object%20Reference) (OtherActor :type Actor%20Object%20Reference) (OtherComp :type Primitive%20Component%20Object%20Reference) (OtherBodyIndex :type Integer)))

(event EventBeginPlay
  (CallFunction|ChangeTrafficLightState))

(event Collision|EventActorBeginOverlap
  (params (OtherActor :type Actor%20Object%20Reference)))

(event EventTick
  (params (DeltaSeconds :type Float%20%28single-precision%29)))

(fn ConstructionScript)

(fn NewFunction)

(fn ChangeTrafficLightState
  (switch Utilities|FlowControl|Switch|SwitchonEtrafficState (Variables|Default|GetTrafficState)
    (:NewEnumerator0
      ;[1 1 1] SENT ROJO
      (Utilities|FlowControl|Sequence
        (:then_0
          (Rendering|SetVisibility (Variables|Default|GetLuzRoja) true false))
        (:then_1
          (Rendering|SetVisibility (Variables|Default|GetLuzAmarilla) false false))
        (:then_2
          (Rendering|SetVisibility (Variables|Default|GetLuzVerde) false false)
          (Variables|Default|SetTrafficState "NewEnumerator2")
          (Development|PrintString " (\"Nuevo estado del semáforo: \" + TrafficState);")
          (Development|PrintString "rOJO")
          (Utilities|Time|SetTimerbyFunctionName 0 "ChangeTrafficLightState" 6.0))))
    (:NewEnumerator1
      ;[1 1 1] sETAMARILLO
      (Utilities|FlowControl|Sequence
        (:then_0
          (Rendering|SetVisibility (Variables|Default|GetLuzRoja) false false))
        (:then_1
          (Rendering|SetVisibility (Variables|Default|GetLuzAmarilla) true false))
        (:then_2
          (Rendering|SetVisibility (Variables|Default|GetLuzVerde) false false)
          (Variables|Default|SetTrafficState "NewEnumerator0")
          (Development|PrintString " (\"Nuevo estado del semáforo: \" + TrafficState);")
          (Development|PrintString "AMARILLO")
          (Utilities|Time|SetTimerbyFunctionName 0 "ChangeTrafficLightState" 2.0))))
    (:NewEnumerator2
      (Utilities|FlowControl|Sequence
        (:then_0
          (Rendering|SetVisibility (Variables|Default|GetLuzRoja) false false))
        (:then_1
          (Rendering|SetVisibility (Variables|Default|GetLuzAmarilla) false false))
        (:then_2
          (Rendering|SetVisibility (Variables|Default|GetLuzVerde) true false)
          (Variables|Default|SetTrafficState "NewEnumerator1")
          (Development|PrintString " (\"Nuevo estado del semáforo: \" + TrafficState);")
          (Development|PrintString "Color ahora es verde")
          (Utilities|Time|SetTimerbyFunctionName 0 "ChangeTrafficLightState" 6.0))))))